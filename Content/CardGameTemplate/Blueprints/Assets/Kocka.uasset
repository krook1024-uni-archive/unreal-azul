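; Kocka ("cube") is an actor in the card game template that the player can drag around with the mouse.
; Its Tipusa ("type") variable sets the cube's material in the construction script and again on BeginPlay, which also enables cursor, click and hover events.
; Hovering shows a hand cursor.
; Click and release open and close a Tick gate that moves the cube to the cursor's trace hit at fixed height, pausing hover events meanwhile.
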(event OnClicked(Kocka)
  (params (TouchedComponent :type Primitive%20Component%20Object%20Reference) (ButtonPressed :type Key%20Structure :default "None"))
  (bind _returnvalue (Game|GetPlayerController 0))
  (bind _hitresult (Game|Player|GetHitResultUnderCursorbyChannel _returnvalue "TraceTypeQuery1" true))
  (bind _location (Collision|BreakHitResult _hitresult))
  (bind (_x _y) (Math|Vector|BreakVector _location))
  (Utilities|FlowControl|Sequence
    (:then_0
      (Utilities|FlowControl|Gate true) ; enters at Open
    )
    (:then_1
      (Variables|/Script/Engine.PlayerController|SetbEnableMouseOverEvents (Game|GetPlayerController 0) false))))

(event OnReleased(Kocka)
  (params (TouchedComponent :type Primitive%20Component%20Object%20Reference) (ButtonReleased :type Key%20Structure :default "None"))
  (bind _returnvalue (Game|GetPlayerController 0))
  (bind _hitresult (Game|Player|GetHitResultUnderCursorbyChannel _returnvalue "TraceTypeQuery1" true))
  (bind _location (Collision|BreakHitResult _hitresult))
  (bind (_x _y) (Math|Vector|BreakVector _location))
  (Utilities|FlowControl|Sequence
    (:then_0
      (Variables|/Script/Engine.PlayerController|SetbEnableMouseOverEvents (Game|GetPlayerController 0) true))
    (:then_1
      (Utilities|FlowControl|Gate true) ; enters at Close
    )))

(event EventBeginPlay
  (bind _returnvalue (Game|GetPlayerController 0))
  (Utilities|FlowControl|Sequence
    (:then_0
      ;[1 1 1] Material beállítása
      (Rendering|Material|SetMaterial (Variables|Default|GetKocka) 0 (Variables|Default|GetTipusa)))
    (:then_1
      (Variables|/Script/Engine.PlayerController|SetbEnableClickEvents (Game|GetPlayerController 0) true))
    (:then_2
      ;[1 1 1] Az egérmutató átváltoztatása kézzé ha a kocka fölé visszük az egeret
      (Variables|/Script/Engine.PlayerController|SetbShowMouseCursor _returnvalue true)
      (Variables|/Script/Engine.PlayerController|SetbEnableMouseOverEvents _returnvalue true))))

(event EventTick
  (params (DeltaSeconds :type Float%20%28single-precision%29))
  (bind _returnvalue (Game|GetPlayerController 0))
  (bind _hitresult (Game|Player|GetHitResultUnderCursorbyChannel _returnvalue "TraceTypeQuery1" true))
  (bind _location (Collision|BreakHitResult _hitresult))
  (bind (_x _y) (Math|Vector|BreakVector _location))
  (Utilities|FlowControl|Gate true
    (:Exit
      ;[1 1 1] Kocka vonszolása az egérrel
      (Transformation|SetWorldLocation (Variables|Default|GetKocka) (Math|Vector|MakeVector _x _y 5e+01) false true))))

(event MouseInput|EventActorBeginCursorOver
  ;[1 1 1] Az egérmutató átváltoztatása kézzé ha a kocka fölé visszük az egeret
  (Variables|/Script/Engine.PlayerController|SetCurrentMouseCursor (Game|GetPlayerController 0) "Hand"))

(event MouseInput|EventActorEndCursorOver
  ;[1 1 1] Az egérmutató átváltoztatása kézzé ha a kocka fölé visszük az egeret
  (Variables|/Script/Engine.PlayerController|SetCurrentMouseCursor (Game|GetPlayerController 0) "Default"))

(fn ConstructionScript
  (Rendering|Material|SetMaterial (Variables|Default|GetKocka) 0 (Variables|Default|GetTipusa)))